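; Player controller that owns the HUD and switches the player between SevenCharacter pawns.
; On BeginPlay it creates the HUD widget and has it build character images, then relays HP, XP and character death updates to it.
; Switching possesses the given character, moves the view target to it and calls its OnPossessed.
; Releasing U makes every EnemyCharacter suicide, and K does the same to the controlled character.
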(event `self.ReceiveBeginPlay`
  (bind _returnvalue (`|CreateWidget` "/Game/UI/WB_HUDWidget.WB_HUDWidget_C"))
  (`UserWidget.AddToViewport` _returnvalue 0)
  (bind _output_get (set `self.HUDWidget` _returnvalue))
  (`/Game/UI/WB_HUDWidget.CreateSevenCharacterImages` _output_get self))

(event `self.SwitchSevenCharacter`
  (params (SevenCharacter :type "SevenCharacter Object Reference"))
  (`self.UnPossess`)
  (`self.Possess` SevenCharacter)
  (`self.SetViewTargetWithBlend` SevenCharacter)
  (`SevenCharacter.OnPossessed` SevenCharacter false))

(event `Key|U`
  (params (Key :type "Key Structure"))
  (:`Released`
    (bind _outactors (`GameplayStatics.GetAllActorsOfClass` "/Script/Seven.EnemyCharacter"))
    (for _array_element _outactors
      (`SevenCharacter.Suicide` _array_element))))

(event `Key|K`
  (params (Key :type "Key Structure"))
  (:`Released`
    (bind _asseven_character (cast `SevenCharacter` (`self.K2_GetPawn`)))
    (`SevenCharacter.Suicide` _asseven_character)))

(event `self.UpdateHPWidget`
  (params (NewHP :type "Float (single-precision)"))
  ;[1 1 1] UI
  (`/Game/UI/WB_HUDWidget.SetHP` (`self.HUDWidget`) NewHP))

(event `self.UpdateXPWidget`
  (params (NewHP :type "Float (single-precision)"))
  ;[1 1 1] UI
  (`/Game/UI/WB_HUDWidget.SetXP` (`self.HUDWidget`) NewHP))

(event `self.UpdateDeadCharacter`
  (params (Name :type "Name (by ref)"))
  ;[1 1 1] UI
  (`/Game/UI/WB_HUDWidget.SetDeadCharacter` (`self.HUDWidget`) (`KismetTextLibrary.Conv_NameToText` Name)))

(fn `UserConstructionScript`)