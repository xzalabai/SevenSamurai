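; BP_Halberd is a character Blueprint that exercises combo, mission, weapon upgrade and character selection systems through hard-coded keys.
; It enables input on BeginPlay, then each key looks up a manager actor by class and calls it.
; H buys a combo, J moves to the mission area, K upgrades this character's weapon, L selects characters.
; Only the ComboManager lookup is validity-checked; spawning and a second combo purchase are unwired.
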(event `self.ReceiveBeginPlay`
  (`self.EnableInput` (`GameplayStatics.GetPlayerController` 0)))

(event `self.ReceiveTick`
  (params (DeltaSeconds :type "Float (single-precision)")))

(event `Key|H`
  (params (Key :type "Key Structure"))
  (:`Released`
    (bind _returnvalue (`GameplayStatics.GetActorOfClass` "/Script/Seven.ComboManager"))
    (`/Engine/EditorBlueprintResources/StandardMacros.IsValid` _returnvalue
      (:`Is Valid`
        (`ComboManager.ShowSkillTree` _returnvalue (`|MakeArray` self :!type "SevenCharacter Object Reference"))
        (`ComboManager.BuyCombo` _returnvalue self 0))
      (:`Is Not Valid`
        (`KismetSystemLibrary.PrintString` "There is no ComboManager" true true (struct :`R` 1.0 :`B` 0.305044 :`A` 1.0))))))

(event `Key|J`
  (params (Key :type "Key Structure"))
  (:`Released`
    (bind _returnvalue (`GameplayStatics.GetActorOfClass` "/Script/Seven.MissionHandler"))
    (`MissionHandler.MovingToMissionArea` _returnvalue)))

(event `Key|K`
  (params (Key :type "Key Structure"))
  (:`Pressed`
    (bind _returnvalue (`GameplayStatics.GetActorOfClass` "/Script/Seven.WeaponUpgrade"))
    (`WeaponUpgrade.ShowPossibleWeaponUpgrades` _returnvalue)
    (`WeaponUpgrade.UpgradeWeapon` _returnvalue self)))

(event `Key|L`
  (params (Key :type "Key Structure"))
  (:`Released`
    (bind _returnvalue (`GameplayStatics.GetActorOfClass` "/Script/Seven.CharacterPicker"))
    (`CharacterPicker.ShowAvailableCharacters` _returnvalue)
    (`CharacterPicker.SelectCharacters` _returnvalue (`|MakeArray` 1 3))
    (`CharacterPicker.ShowSelectedCharacters` _returnvalue)))

(fn `UserConstructionScript`)