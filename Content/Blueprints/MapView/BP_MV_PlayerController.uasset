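; Player controller for the map view, handling map clicks, level return and camp toggling.
; On BeginPlay it possesses the BP_DefaultCamera found in the level, and releasing the left mouse button calls PerformTraceToMap, which is defined outside this graph.
; Releasing E opens the Map level when the current level is VillageView.
; Pressing C alternates Camp on and off on MVSevenCharacter through a FlipFlop.
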(event `self.ReceiveBeginPlay`
  (`|ExecutionSequence`
    (:`then_0`
      (bind _returnvalue (`GameplayStatics.GetActorOfClass` "/Game/Blueprints/MapView/BP_DefaultCamera.BP_DefaultCamera_C"))
      (`self.Possess` _returnvalue))))

(event `Key|LeftMouseButton`
  (params (Key :type "Key Structure"))
  (:`Released`
    (`self.PerformTraceToMap`)))

(event `Key|E`
  (params (Key :type "Key Structure"))
  (:`Released`
    (bind _returnvalue (`GameplayStatics.GetCurrentLevelName` true))
    (if (`KismetStringLibrary.EqualEqual_StrStr` "VillageView" _returnvalue)
      (`GameplayStatics.OpenLevel` "Map"))))

(event `Key|C`
  (params (Key :type "Key Structure"))
  (bind _mvsevencharacter (`self.MVSevenCharacter`))
  (:`Pressed`
    (`/Engine/EditorBlueprintResources/StandardMacros.FlipFlop`
      (:`A`
        (`MVSevenCharacter.Camp` _mvsevencharacter true))
      (:`B`
        (`MVSevenCharacter.Camp` _mvsevencharacter false)))))

(fn `UserConstructionScript`)